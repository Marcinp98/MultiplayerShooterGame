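; BP_ShooterCharacter is the shooter character Blueprint, which shows the player's name on an overhead widget.
; On BeginPlay it polls every 0.2 seconds until PlayerState is valid, since it may not be available at spawn.
; It then casts the OverheadWidget component's widget to WBP_OverheadWidget and calls ShowPlayerName with itself.
; A net role display call remains in the graph but is disconnected, and Tick and overlap events are empty.
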(event `self.ReceiveBeginPlay`
  ;[1 1 1] Showing NetRole and Name
  (`KismetSystemLibrary.Delay` 0.2 :!label _label)
  (if (`KismetSystemLibrary.IsValid` (`self.PlayerState`))
    (bind _aswbp_overhead_widget (cast `/Game/Blueprints/HUD/WBP_OverheadWidget` (`WidgetComponent.GetUserWidgetObject` (`self.OverheadWidget`))))
    (`OverheadWidget.ShowPlayerName` _aswbp_overhead_widget self)
    (else
      (goto _label))))

(fn `UserConstructionScript`)